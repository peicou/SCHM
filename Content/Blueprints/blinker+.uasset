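; Short-lived helper actor that restores an LED color on the SCHM_UI_main UI after a brief delay.
; Its construction script caches the first SCHM_UI_main actor found and starts a timer by function name.
; When the timer fires, restoreColor applies the stored BlinkerColor to BlinkerLED through SetLEDColor, then the actor destroys itself.
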(fn ConstructionScript
  (bind _outactors (Actor|GetAllActorsOfClass "/Game/Blueprints/SCHM_UI_main+.SCHM_UI_main+_C"))
  (Variables|Default|SetuiRef (Utilities|Array|Get(acopy) _outactors))
  (Utilities|Time|SetTimerbyFunctionName self "restoreColor" 0.3))

(fn RestoreColor
  (Default|SetLEDColor (Variables|Default|GetuiRef) (Variables|Default|GetblinkerColor) (Variables|Default|GetblinkerLED))
  (Actor|DestroyActor))