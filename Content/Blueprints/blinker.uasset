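; A short-lived actor that sets an LED color on the SCHM_UI_main actor after a brief delay, serving as one timed step of a blink.
; Its construction script caches the first SCHM_UI_main found in the world and starts a timer for restoreColor.
; When the timer fires, restoreColor applies BlinkerColor to BlinkerLED through SetLEDColor, then the actor destroys itself.
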(fn ConstructionScript
  (bind _outactors (Actor|GetAllActorsOfClass "/Game/Blueprints/SCHM_UI_main.SCHM_UI_main_C"))
  (Variables|Default|SetuiRef (Utilities|Array|Get(acopy) _outactors))
  (Utilities|Time|SetTimerbyFunctionName self "restoreColor" 0.3))

(fn RestoreColor
  (Default|SetLEDColor (Variables|Default|GetuiRef) (Variables|Default|GetblinkerColor) (Variables|Default|GetblinkerLED))
  (Actor|DestroyActor))