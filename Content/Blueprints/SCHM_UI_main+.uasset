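; Main UI actor for a device panel with LEDs and a PIN screen, enabling game-and-UI input and blacking out the screen on BeginPlay.
; LED and backlight colors are set through the LEDColor parameter on dynamic materials.
; BlinkLed applies a new color and spawns a Blinker actor holding the previous color, LED and time.
; ShowUI and HideUI toggle component visibility and shift components along Y.
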(event Custom|setLEDColor
  (params (color :type Linear%20Color%20Structure) (LED :type Integer :default 0))
  (Rendering|Material|SetVectorParameterValue (Variables|/Game/Blueprints/LEDLight.LEDLight_C|GetLEDColorDynMat (Utilities|Array|Get(acopy) (Variables|Default|GetLEDs) LED)) "LEDColor" color :!class /Script/Engine.MaterialInstanceDynamic))

(event Custom|setPINScreenColor
  (params (color :type Linear%20Color%20Structure))
  (Rendering|Material|SetVectorParameterValue (Variables|/Game/Blueprints/pinScreenBacklight.pinScreenBacklight_C|GetbacklightDynMat (Variables|Default|GetpinScreen)) "LEDColor" color :!class /Script/Engine.MaterialInstanceDynamic))

(event EventBeginPlay
  (Input|SetInputModeGameandUI (Game|GetPlayerController 0) 0 false true)
  (CallFunction|SetPINScreenColor "(R=0.000000,G=0.000000,B=0.000000,A=1.000000)"))

(fn ConstructionScript
  (Variables|Default|SetmyListContent "Item List"))

(fn WatchString
  (return (Variables|Default|Getupdate)))

(fn ShowUI
  (params (UI :type Widget%20Component%20Object%20Reference))
  (bind _relativelocation (Variables|/Script/Engine.SceneComponent|GetRelativeLocation UI))
  (bind (_x _y _z) (Math|Vector|BreakVector _relativelocation))
  (Rendering|SetVisibility UI true true)
  (Development|SetHiddeninGame UI false false)
  (Transformation|SetRelativeLocation UI (Math|Vector|MakeVector _x 0.0 _z) false))

(fn HideUI
  (params (UI :type Widget%20Component%20Object%20Reference))
  (bind _relativelocation (Variables|/Script/Engine.SceneComponent|GetRelativeLocation UI))
  (bind (_x _y _z) (Math|Vector|BreakVector _relativelocation))
  (Rendering|SetVisibility UI false true)
  (Transformation|SetRelativeLocation UI (Math|Vector|MakeVector _x -1e+01 _z) false)
  (Development|SetHiddeninGame UI false false))

(fn BlinkLed
  (params (LED :type Integer :default 0) (Time :type Float%20%28single-precision%29 :default 0.0) (Color :type Linear%20Color%20Structure))
  (bind _returnvalue (Rendering|Material|GetVectorParameterValue (Variables|/Game/Blueprints/LEDLight.LEDLight_C|GetLEDColorDynMat (Utilities|Array|Get(acopy) (Variables|Default|GetLEDs) LED)) "LEDColor" :!class /Script/Engine.MaterialInstanceDynamic))
  (bind _returnvalue_2 (Game|SpawnActorfromClass "/Game/Blueprints/blinker+.blinker+_C" (Variables|Default|Getlocation) false 0))
  (Variables|/Game/Blueprints/blinker+.blinker+_C|SetblinkerColor _returnvalue_2 _returnvalue)
  (Variables|/Game/Blueprints/blinker+.blinker+_C|SetblinkerLED _returnvalue_2 LED)
  (Variables|/Game/Blueprints/blinker+.blinker+_C|SetblinkerTime _returnvalue_2 Time)
  (CallFunction|SetLEDColor Color LED))